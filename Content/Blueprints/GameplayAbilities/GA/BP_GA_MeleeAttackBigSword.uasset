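; Gameplay ability for a big-sword melee attack, using the weapon equipped in the avatar's WeaponsManagerComponent and ending at once if none is valid.
; It plays a horizontal swing montage and ends when that completes, is interrupted or is cancelled.
; On authority, HitScan Start/End gameplay events open and close the weapon's hit scan, passing an instant-damage effect spec with SetByCaller damage.
; Ending the ability also stops the hit scan as a safeguard.
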(event `self.K2_ActivateAbility`
  (bind _returnvalue (`Actor.GetComponentByClass` (`self.GetAvatarActorFromActorInfo`) "/Game/Blueprints/Weapons/Sword/WeaponsManagerComponent.WeaponsManagerComponent_C"))
  (`/Engine/EditorBlueprintResources/StandardMacros.IsValid` _returnvalue
    (:`Is Valid`
      (bind _equippedweapon (`/Game/Blueprints/Weapons/Sword/WeaponsManagerComponent.EquippedWeapon` _returnvalue)
        (:`then`
          (set `self.Equipped Weapon` _equippedweapon)
          (`AbilityTask_PlayMontageAndWait.CreatePlayMontageAndWaitProxy` "None" "/Game/Blueprints/Characters/MainCharacter/Animations/AnimSequences/StandingMeleeAttackHorizontal_1__UE_Anim_Montage.StandingMeleeAttackHorizontal_1__UE_Anim_Montage" 1.0 "None" true 1.0 0.0 true
            (:`then`
              (`self.K2_HasAuthority`
                (:`True`
                  (`AbilityTask_WaitGameplayEvent.WaitGameplayEvent` (struct :`TagName` "Event.HitScan.Start") null
                    (:`then`
                      (`AbilityTask_WaitGameplayEvent.WaitGameplayEvent` (struct :`TagName` "Event.HitScan.End") null
                        (:`EventReceived`
                          (bind _equipped_weapon (`self.Equipped Weapon`)
                            (:`then`
                              (`/Game/Blueprints/Weapons/Sword/BP_WeaponBase.HitScanEnd` _equipped_weapon))
                            (:`else`)))))
                    (:`EventReceived`
                      ;[0 0.15 0.004452 0.5] Нанесение урона
                      (bind _equipped_weapon_2 (`self.Equipped Weapon`)
                        (:`then`
                          (bind _returnvalue_2 (`AbilitySystemBlueprintLibrary.AssignTagSetByCallerMagnitude` (`self.MakeOutgoingGameplayEffectSpec` "/Game/Blueprints/GameplayAbilities/GE/GE_InstantDamage.GE_InstantDamage_C") (struct :`TagName` "Data.Damage") (`self.Damage`)))
                          (`/Game/Blueprints/Weapons/Sword/BP_WeaponBase.HitScanStart` _equipped_weapon_2 _returnvalue_2))
                        (:`else`)))))))
            (:`OnCompleted`
              (`self.K2_EndAbility` :!label _label))
            (:`OnInterrupted`
              (goto _label))
            (:`OnCancelled`
              (goto _label))))
        (:`else`
          (`self.K2_EndAbility` :!label _label_2))))
    (:`Is Not Valid`
      (goto _label_2))))

(event `self.K2_OnEndAbility`
  (params (bWasCancelled :type Boolean))
  ;[0 0.15 0.01771 0.5] Это на всякий случай
  (bind _equipped_weapon (`self.Equipped Weapon`)
    (:`then`
      (`/Game/Blueprints/Weapons/Sword/BP_WeaponBase.HitScanEnd` _equipped_weapon))
    (:`else`)))