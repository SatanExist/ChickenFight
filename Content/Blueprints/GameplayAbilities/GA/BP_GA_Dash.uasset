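; Gameplay ability that dashes BP_MainCharacter in its current direction of movement.
; On activation it commits the cost, then applies a very brief, strong root motion constant force along the avatar's velocity, keeping the final velocity afterwards.
; A dash gameplay cue runs until the ability ends.
; The cooldown is committed only when the force finishes, just before the ability ends.
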(event `self.K2_ActivateAbility`
  (`KismetSystemLibrary.PrintString` "DASH")
  (`self.K2_CommitAbilityCost` false)
  (bind _asbp_main_character (cast `/Game/Blueprints/Characters/MainCharacter/BP_MainCharacter` (`self.GetAvatarActorFromActorInfo`)))
  (set `self.As BP Main Character` _asbp_main_character)
  (`AbilityTask_ApplyRootMotionConstantForce.ApplyRootMotionConstantForce` "None" (`Actor.GetVelocity` (`self.As BP Main Character`)) 4000.0 0.02 false null "MaintainLastRootMotionVelocity"
    (:`then`
      (`self.K2_AddGameplayCue` (struct :`TagName` "GameplayCue.Dash.Active")))
    (:`OnFinish`
      (`self.K2_CommitAbilityCooldown` false)
      (`self.K2_EndAbility`))))