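; Gameplay ability that equips or unequips the avatar's weapon based on a gameplay event.
; It switches on the event's first target tag, telling the avatar's WeaponsManagerComponent to equip BP_Sword for the Big Sword tag or unequip for any other.
; The ability ends right after the switch, but EndAbility is not reached when the avatar lacks that component.
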(event `self.K2_ActivateAbilityFromEvent`
  (params (EventData :type "GameplayEventData Structure (by ref)"))
  (bind _returnvalue (`Actor.GetComponentByClass` (`self.GetAvatarActorFromActorInfo`) "/Game/Blueprints/Weapons/Sword/WeaponsManagerComponent.WeaponsManagerComponent_C"))
  (`/Engine/EditorBlueprintResources/StandardMacros.IsValid` _returnvalue
    (:`Is Valid`
      (`|ExecutionSequence`
        (:`then_0`
          (`|SwitchGameplayTag` (`|GetArrayItem` (`BlueprintGameplayTagLibrary.BreakGameplayTagContainer` (`.TargetTags` (break `GameplayEventData` EventData))))
            (:`Default`
              (`/Game/Blueprints/Weapons/Sword/WeaponsManagerComponent.UnequipWeapon` _returnvalue))
            (:`Weapon.Melee.BigSword`
              (`/Game/Blueprints/Weapons/Sword/WeaponsManagerComponent.EquipWeapon` _returnvalue "/Game/Blueprints/Weapons/Sword/BP_Sword.BP_Sword_C"))))
        (:`then_1`
          (`self.K2_EndAbility`))))))