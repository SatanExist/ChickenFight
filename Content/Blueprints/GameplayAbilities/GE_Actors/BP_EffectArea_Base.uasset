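; Base effect area actor that applies a configurable Gameplay Effect to overlapping actors that have an Ability System Component.
; On begin overlap, it builds a spec from the effect class with itself as causer, sets a tagged SetByCaller magnitude, and applies it to that actor.
; On end overlap, it removes all stacks of that effect class, which suits infinite effects such as damage over time.
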(event `self.ReceiveActorBeginOverlap`
  (params (OtherActor :type "Actor Object Reference"))
  (bind _returnvalue (`AbilitySystemBlueprintLibrary.GetAbilitySystemComponent` OtherActor))
  (`/Engine/EditorBlueprintResources/StandardMacros.IsValid` _returnvalue
    (:`Is Valid`
      ;[0 0.15 0.002167 0.5] Итак, я хочу применить эффектор и произвести вычисление, например нанесение урона ( в моем случае GE_DamageOverTime_Infinite )
      (bind _returnvalue_2 (`AbilitySystemBlueprintLibrary.MakeSpecHandleByClass` (`self.EffectClass`) null self))
      (bind _returnvalue_3 (`AbilitySystemBlueprintLibrary.AssignTagSetByCallerMagnitude` _returnvalue_2 (`self.EffectMagnitudeDataTag`) (`self.EffectMagnitudeValue`)))
      (`AbilitySystemComponent.BP_ApplyGameplayEffectSpecToSelf` _returnvalue _returnvalue_3))))

(event `self.ReceiveActorEndOverlap`
  (params (OtherActor :type "Actor Object Reference"))
  (bind _returnvalue (`AbilitySystemBlueprintLibrary.GetAbilitySystemComponent` OtherActor))
  (`/Engine/EditorBlueprintResources/StandardMacros.IsValid` _returnvalue
    (:`Is Valid`
      ;[0.002764 0.15 0.002321 0.5] Отменить действие эффектора ( он бесконечный )
      (`AbilitySystemComponent.RemoveActiveGameplayEffectBySourceEffect` _returnvalue (`self.EffectClass`) null -1))))

(fn `UserConstructionScript`)