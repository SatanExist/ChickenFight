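; Main character Blueprint built on the Gameplay Ability System, handling attributes, combat input and death.
; BeginPlay seeds health and stamina through a SetByCaller effect, then listens for attribute changes.
; Stamina loss restarts a regen effect after a short delay until full, while zero health strips abilities and ragdolls the mesh.
; Key 1 sends a big-sword equip event and Space triggers its melee attack; the Dash grant and activation nodes are disconnected.
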(event `Key|One`
  (params (Key :type "Key Structure"))
  (:`Pressed`
    (`AbilitySystemBlueprintLibrary.SendGameplayEventToActor` self (struct :`TagName` "Event.Weapon.Equip") (make `GameplayEventData` (struct) null null null null (struct) (struct) (struct :`GameplayTags` (struct :`(TagName` "Weapon.Melee.BigSword")))))))

(event `self.ReceiveBeginPlay`
  ;[0.005333 0.15 0 0.5] Инициализация начальных данных для персонажа через Effector
  (bind _returnvalue (`AbilitySystemBlueprintLibrary.MakeSpecHandleByClass` "/Game/Blueprints/Characters/MainCharacter/GE_Initial_MainCharacter.GE_Initial_MainCharacter_C" self))
  (bind _returnvalue_2 (`AbilitySystemBlueprintLibrary.AssignTagSetByCallerMagnitude` _returnvalue (struct :`TagName` "Data.Initial.MainCharacter.MaxHealth") 300.0))
  (`AbilitySystemComponent.BP_ApplyGameplayEffectSpecToSelf` (`self.ASC_AbilitySystemComponent`) _returnvalue_2)
  (bind _returnvalue_3 (`AbilitySystemBlueprintLibrary.AssignTagSetByCallerMagnitude` _returnvalue (struct :`TagName` "Data.Initial.MainCharacter.Health") 300.0))
  (`AbilitySystemComponent.BP_ApplyGameplayEffectSpecToSelf` (`self.ASC_AbilitySystemComponent`) _returnvalue_3)
  (bind _returnvalue_4 (`AbilitySystemBlueprintLibrary.AssignTagSetByCallerMagnitude` _returnvalue (struct :`TagName` "Data.Initial.MainCharacter.MaxStamina") 100.0))
  (`AbilitySystemComponent.BP_ApplyGameplayEffectSpecToSelf` (`self.ASC_AbilitySystemComponent`) _returnvalue_4)
  (bind _returnvalue_5 (`AbilitySystemBlueprintLibrary.AssignTagSetByCallerMagnitude` _returnvalue (struct :`TagName` "Data.Initial.MainCharacter.Stamina") 100.0))
  (`AbilitySystemComponent.BP_ApplyGameplayEffectSpecToSelf` (`self.ASC_AbilitySystemComponent`) _returnvalue_5)
  ;[0.0155 0.15 0.01158 0.5] Функция слушатель, которая проверяет постоянно атрибут на изменения
  (bind (_asynctaskproxy _attribute _newvalue _oldvalue) (`AbilityAsync_WaitAttributeChanged.WaitForAttributeChanged` null (struct :`AttributeName` "Stamina" :`Attribute` "/Script/ChickenFight.GA_AttributeSet:Stamina" :`AttributeOwner` "/Script/CoreUObject.Class'/Script/ChickenFight.GA_AttributeSet'"))
    (:`then`
      (bind (_asynctaskproxy_2 _attribute_2 _newvalue_2) (`AbilityAsync_WaitAttributeChanged.WaitForAttributeChanged` null (struct :`AttributeName` "Health" :`Attribute` "/Script/ChickenFight.GA_AttributeSet:Health" :`AttributeOwner` "/Script/CoreUObject.Class'/Script/ChickenFight.GA_AttributeSet'"))
        (:`Changed`
          (`self.DieEvent` _newvalue_2))))
    (:`Changed`
      (`self.HandleStaminaChanged` _newvalue _oldvalue))))

(event `DieEvent`
  (params (NewHelath :type "Float (double-precision)"))
  (if (<= NewHelath 0.0)
    (`self.DieFunction`)))

(event `HandleStaminaChanged`
  (params (NewValue :type "Float (double-precision)") (OldValue :type "Float (double-precision)"))
  (bind (_maxstamina_basevalue _maxstamina_currentvalue) (break `GameplayAttributeData` (`GA_AttributeSet.MaxStamina` (`self.GA_AS_AttributeSet`))))
  ;[0.0155 0.15 0.01158 0.5] Функция слушатель, которая проверяет постоянно атрибут на изменения
  (if (< NewValue OldValue)
    ;;[0.15 0 0.1272 0.5] Танцы с бубном чтоб всё работало
    (`AbilitySystemComponent.RemoveActiveEffectsWithTags` (`self.ASC_AbilitySystemComponent`) (struct :`GameplayTags` (struct :`(TagName` "Status.Stamina.Regen"))))
    (`KismetSystemLibrary.Delay` 0.5)
    ;;[0.00838 0.276 0] Применение Эффекта GE
    (`AbilitySystemComponent.BP_ApplyGameplayEffectToSelf` :`self` (`self.ASC_AbilitySystemComponent`) :`GameplayEffectClass` "/Game/Blueprints/GameplayAbilities/GE/GE_Status_StaminaRegen.GE_Status_StaminaRegen_C")
    (elif (>= NewValue _maxstamina_currentvalue)
      ;;[0.00838 0.276 0] Отмена Эффекта GE по тегу
      (`AbilitySystemComponent.RemoveActiveEffectsWithTags` (`self.ASC_AbilitySystemComponent`) (struct :`GameplayTags` (struct :`(TagName` "Status.Stamina.Regen")))))))

(event `Key|SpaceBar`
  (params (Key :type "Key Structure"))
  (:`Pressed`
    (`AbilitySystemComponent.TryActivateAbilityByClass` (`self.ASC_AbilitySystemComponent`) "/Game/Blueprints/GameplayAbilities/GA/BP_GA_MeleeAttackBigSword.BP_GA_MeleeAttackBigSword_C" true)))

(fn `DieFunction`
  (bind _outabilityhandles (`AbilitySystemComponent.GetAllAbilities` (`self.ASC_AbilitySystemComponent`)))
  (`self.RemoveAbilities` _outabilityhandles)
  (`CharacterMovementComponent.DisableMovement` (`self.CharacterMovement`))
  (`MovementComponent.StopMovementImmediately` (`self.CharacterMovement`))
  (`PrimitiveComponent.SetCollisionProfileName` (`self.Mesh`) "Ragdoll" true)
  (`PrimitiveComponent.SetSimulatePhysics` (`self.Mesh`) true))

(fn `UserConstructionScript`)