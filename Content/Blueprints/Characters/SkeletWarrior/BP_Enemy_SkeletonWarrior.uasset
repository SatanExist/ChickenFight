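; Skeleton warrior enemy built on GAS, with attack and take-damage abilities, a health bar and health regeneration.
; BeginPlay grants the abilities, initializes health through a SetByCaller effect spec, and starts attribute listeners that update the widget, set a looping bones-sound timer and check health.
; Damage removes the regen effect and reapplies it after a short delay.
; Death strips abilities, hides the bar, ragdolls the mesh with an upward impulse, then destroys the actor.
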(event `self.ReceiveBeginPlay`
  (bind _asc_abilitysystemcomponent (`self.ASC_AbilitySystemComponent`))
  (`AbilitySystemComponent.K2_GiveAbility` (`self.ASC_AbilitySystemComponent`) "/Game/Blueprints/Characters/SkeletWarrior/BaseGameplaythings/GA_TakeDamage.GA_TakeDamage_C" 0 -1)
  (`AbilitySystemComponent.K2_GiveAbility` (`self.ASC_AbilitySystemComponent`) "/Game/Blueprints/Characters/SkeletWarrior/BaseGameplaythings/GA_AttackHero.GA_AttackHero_C" 0 -1)
  (bind _returnvalue (`AbilitySystemBlueprintLibrary.MakeSpecHandleByClass` "/Game/Blueprints/Characters/SkeletWarrior/GE_Initial_SkeletonWarrior.GE_Initial_SkeletonWarrior_C" self))
  (bind _returnvalue_2 (`AbilitySystemBlueprintLibrary.AssignTagSetByCallerMagnitude` _returnvalue (struct :`TagName` "Data.Initial.SkeletonWarrior.MaxHealth") 27.0))
  (`AbilitySystemComponent.BP_ApplyGameplayEffectSpecToSelf` (`self.ASC_AbilitySystemComponent`) _returnvalue_2)
  (bind _returnvalue_3 (`AbilitySystemBlueprintLibrary.AssignTagSetByCallerMagnitude` _returnvalue (struct :`TagName` "Data.Initial.SkeletonWarrior.Health") 27.0))
  (`AbilitySystemComponent.BP_ApplyGameplayEffectSpecToSelf` (`self.ASC_AbilitySystemComponent`) _returnvalue_3)
  (bind (_asynctaskproxy _attribute _newvalue _oldvalue) (`AbilityAsync_WaitAttributeChanged.WaitForAttributeChanged` null (struct :`AttributeName` "Health" :`Attribute` "/Script/ChickenFight.GA_AttributeSet:Health" :`AttributeOwner` "/Script/CoreUObject.Class'/Script/ChickenFight.GA_AttributeSet'"))
    (:`then`
      (set `self.Health` (`.ReturnValue` (`AbilitySystemBlueprintLibrary.GetFloatAttributeFromAbilitySystemComponent` _asc_abilitysystemcomponent (struct :`AttributeName` "Health" :`Attribute` "/Script/ChickenFight.GA_AttributeSet:Health" :`AttributeOwner` "/Script/CoreUObject.Class'/Script/ChickenFight.GA_AttributeSet'"))))
      (set `self.MaxHealth` (`.ReturnValue` (`AbilitySystemBlueprintLibrary.GetFloatAttributeFromAbilitySystemComponent` _asc_abilitysystemcomponent (struct :`AttributeName` "MaxHealth" :`Attribute` "/Script/ChickenFight.GA_AttributeSet:MaxHealth" :`AttributeOwner` "/Script/CoreUObject.Class'/Script/ChickenFight.GA_AttributeSet'"))))
      (`self.UpdateHealthPercent`)
      ;[0 0.15 0.00732 0.5] Слушатель для обновления здоровья
      (bind (_asynctaskproxy_2 _attribute_2 _newvalue_2) (`AbilityAsync_WaitAttributeChanged.WaitForAttributeChanged` null (struct :`AttributeName` "Health" :`Attribute` "/Script/ChickenFight.GA_AttributeSet:Health" :`AttributeOwner` "/Script/CoreUObject.Class'/Script/ChickenFight.GA_AttributeSet'"))
        (:`Changed`
          (set `self.Health` _newvalue_2)
          (`self.UpdateHealthPercent`)
          (`KismetSystemLibrary.K2_SetTimerDelegate` (delegate `BonesSoundEvent`) 4.0 true))))
    (:`Changed`
      (`self.CheckHealth` _newvalue _oldvalue))))

(event `BonesSoundEvent`
  (`GameplayStatics.PlaySound2D` null 1.0 1.0 0.0 null null))

(event `CheckHealth`
  (params (CurrentHealth :type "Float (double-precision)") (OldValue :type "Float (double-precision)"))
  (bind (_maxhealth_basevalue _maxhealth_currentvalue) (break `GameplayAttributeData` (`GA_AttributeSet.MaxHealth` (`self.GA_AS_AttributeSet`))))
  (if (<= CurrentHealth 0.0)
    (`GameplayStatics.PlaySound2D` "/Game/Blueprints/Characters/SkeletWarrior/SkeletonSounds/skeleton-sounds-2.skeleton-sounds-2" 3.0 1.0 0.5 null null)
    (`SceneComponent.SetVisibility` (`self.Widget`) false false)
    (bind _outabilityhandles (`AbilitySystemComponent.GetAllAbilities` (`self.ASC_AbilitySystemComponent`)))
    (`self.RemoveAbilities` _outabilityhandles)
    (`CharacterMovementComponent.DisableMovement` (`self.CharacterMovement`))
    (`MovementComponent.StopMovementImmediately` (`self.CharacterMovement`))
    (`PrimitiveComponent.SetCollisionProfileName` (`self.Mesh`) "Ragdoll" true)
    (`PrimitiveComponent.SetSimulatePhysics` (`self.Mesh`) true)
    (`PrimitiveComponent.SetCollisionResponseToChannel` (`self.Mesh`) "ECC_Pawn" "ECR_Ignore")
    (`PrimitiveComponent.SetCollisionResponseToChannel` (`self.CapsuleComponent`) "ECC_Pawn" "ECR_Ignore")
    (`PrimitiveComponent.SetCollisionResponseToChannel` (`self.Mesh`) "ECC_GameTraceChannel1" "ECR_Ignore")
    (`PrimitiveComponent.SetCollisionResponseToChannel` (`self.CapsuleComponent`) "ECC_GameTraceChannel1" "ECR_Ignore")
    (`PrimitiveComponent.AddImpulse` (`self.Mesh`) (0.0 0.0 6000.0) "None" true)
    (`KismetSystemLibrary.Delay` 5.0)
    (`self.K2_DestroyActor`)
    (elif (< CurrentHealth OldValue)
      ;[0.15 0 0.1272 0.5] Танцы с бубном чтоб всё работало
      (`AbilitySystemComponent.RemoveActiveEffectsWithTags` (`self.ASC_AbilitySystemComponent`) (struct :`GameplayTags` (struct :`(TagName` "Status.Health.Regen"))))
      (`KismetSystemLibrary.Delay` 0.5)
      ;[0.00838 0.276 0] Применение Эффекта GE
      (`AbilitySystemComponent.BP_ApplyGameplayEffectToSelf` :`self` (`self.ASC_AbilitySystemComponent`) :`GameplayEffectClass` "/Game/Blueprints/GameplayAbilities/GE/GE_Status_HealthRegen.GE_Status_HealthRegen_C")
      (elif (>= 0.0 _maxhealth_currentvalue)
        ;[0.00838 0.276 0] Отмена Эффекта GE по тегу
        (`AbilitySystemComponent.RemoveActiveEffectsWithTags` (`self.ASC_AbilitySystemComponent`) (struct :`GameplayTags` (struct :`(TagName` "Status.Health.Regen"))))))))

(fn `UpdateHealthPercent`
  (bind _aswbp_enemy_health_bar (cast `/Game/Blueprints/Characters/SkeletWarrior/WBP_EnemyHealthBar` (`WidgetComponent.GetWidget` (`self.Widget`))))
  (`ProgressBar.SetPercent` (`/Game/Blueprints/Characters/SkeletWarrior/WBP_EnemyHealthBar.HealthBar` _aswbp_enemy_health_bar) (/ (`self.Health`) (`self.MaxHealth`))))

(fn `UserConstructionScript`)