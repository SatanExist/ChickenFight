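; Base melee weapon Blueprint that detects hits on pawns and applies Gameplay Ability System effects to them.
; HitScanStart stores an effect spec, clears the hit list and starts a looping timer for HitScan, which HitScanEnd stops.
; Each scan sphere-traces between the start and end scene points, ignoring the Instigator.
; Each new target with an ability system receives the effect once per window and attempts to activate GA_TakeDamage.
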(event `HitScan`
  ;[0 0.15 0.01036 0.5] Механизм скана
  (`KismetSystemLibrary.PrintString` "scan")
  (bind _outhits (`KismetSystemLibrary.SphereTraceMultiForObjects` (`SceneComponent.K2_GetComponentLocation` (`self.Scene(TraceStart)`)) (`SceneComponent.K2_GetComponentLocation` (`self.Scene(TraceEnd)`)) (`self.HitScanRadius`) (`|MakeArray` "ObjectTypeQuery3" :!type "EObjectTypeQuery Enum") false (`|MakeArray` (`self.Instigator`) :!type "Actor Object Reference") "None" true (struct :`R` 1.0 :`A` 1.0) (struct :`G` 1.0 :`A` 1.0) 0.1))
  ;[0 0.5156 0.005888 0.5] Получаем засканенных акторов и добавляем в массив, применяем к каждому актору логику (урона в моем случае через ApplyGameplayEffectSpecToSelf )
  (for _array_element _outhits
    (bind (_bblockinghit _binitialoverlap _time _distance _location _impactpoint _normal _impactnormal _physmat _hitactor) (`GameplayStatics.BreakHitResult` _array_element))
    (bind _returnvalue (`AbilitySystemBlueprintLibrary.GetAbilitySystemComponent` _hitactor))
    (`/Engine/EditorBlueprintResources/StandardMacros.IsValid` _returnvalue
      (:`Is Valid`
        (if (not (`KismetArrayLibrary.Array_Contains` (`self.HittedActors`) _hitactor))
          (`KismetArrayLibrary.Array_AddUnique` (`self.HittedActors`) _hitactor)
          (`AbilitySystemComponent.BP_ApplyGameplayEffectSpecToSelf` _returnvalue (`self.EffectSpecHandle`))
          (`AbilitySystemComponent.TryActivateAbilityByClass` _returnvalue "/Game/Blueprints/Characters/SkeletWarrior/BaseGameplaythings/GA_TakeDamage.GA_TakeDamage_C" true))))))

(event `HitScanStart`
  (params (EffectSpecHandle :type "GameplayEffectSpecHandle Structure"))
  ;[0.004248 0.15 0 0.5] Применяем HitScan event в таймере много раз
  (set `self.EffectSpecHandle` EffectSpecHandle)
  (`KismetArrayLibrary.Array_Clear` (`self.HittedActors`))
  (bind _returnvalue (`KismetSystemLibrary.K2_SetTimerDelegate` (`|CreateDelegate` :!event `HitScan`) 0.033333 true))
  (set `self.HitScanTimer` _returnvalue))

(event `HitScanEnd`
  ;[0.001153 0.15 0 0.5] Вырубаем скан
  (`KismetSystemLibrary.K2_ClearAndInvalidateTimerHandle` (`self.HitScanTimer`)))

(fn `UserConstructionScript`)